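; BP_Activator is an activator actor that triggers its list of Interactables when the player presses F.
; It enables input from player controller 0 at BeginPlay, so the key works without any proximity check.
; A press restarts the skeletal mesh animation unless already playing, waits a configurable delay, then calls Activate on each entry in Interactables.
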(event EventBeginPlay
  (Input|EnableInput (Game|GetPlayerController 0)))

(event Collision|EventActorBeginOverlap
  (params (OtherActor :type Actor%20Object%20Reference)))

(event EventTick
  (params (DeltaSeconds :type Float%20%28single-precision%29)))

(event Input|KeyboardEvents|F
  (params (Key :type Key%20Structure :default "None"))
  (:Pressed
    (CallFunction|Activate)
    (Utilities|FlowControl|Delay (Variables|Default|Getdelay))
    (for _array_element (Variables|Default|GetInteractables)
      (Default|Activate _array_element))))

(fn ConstructionScript)

(fn Activate
  (bind _skeletalmesh (Variables|Default|GetSkeletalMesh))
  (if (not (Audio|Components|Audio|IsPlaying _skeletalmesh))
    (Components|Animation|SetPosition _skeletalmesh 0.0 true)
    (Audio|Components|Audio|Play _skeletalmesh false)))