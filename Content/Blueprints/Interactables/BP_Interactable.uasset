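; Interactable Blueprint that plays a skeletal mesh animation when Activate is called, ignoring calls while it is playing.
; With StopAtPosition set, Tick uses a DoOnce to halt and snap the animation at that point, creating a two-stage interaction.
; The next activation resumes past the stop, and one made beyond it rewinds and re-arms the stop.
; Without a stop position, each activation rewinds before playing unless PlayOnce is set.
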(event Custom|Reset%20Stop
  (bind _skeletalmesh (Variables|Default|GetSkeletalMesh))
  (Utilities|FlowControl|DoOnce false) ; enters at Reset
)

(event EventTick
  (params (DeltaSeconds :type Float%20%28single-precision%29))
  (bind _skeletalmesh (Variables|Default|GetSkeletalMesh))
  (if (> (Variables|Interaction|GetstopAtPosition) 0.0)
    (if (>= (Class|SkeletalMeshComponent|GetPosition _skeletalmesh) (Variables|Interaction|GetstopAtPosition))
      (Utilities|FlowControl|DoOnce false
        (:Completed
          (Audio|Components|Audio|Stop _skeletalmesh)
          (Components|Animation|SetPosition _skeletalmesh (Variables|Interaction|GetstopAtPosition) true))))))

(fn ConstructionScript)

(fn Activate
  (bind _skeletalmesh (Variables|Default|GetSkeletalMesh))
  (if (not (Audio|Components|Audio|IsPlaying _skeletalmesh))
    (if (> (Variables|Interaction|GetstopAtPosition) 0.0)
      (if (not (> (Class|SkeletalMeshComponent|GetPosition _skeletalmesh) (Variables|Interaction|GetstopAtPosition)))
        _
        (else
          (Components|Animation|SetPosition _skeletalmesh 0.0 true :!label _label)
          (CallFunction|ResetStop)))
      (elif (not (Variables|Interaction|GetplayOnce))
        (goto _label)
        (else
          _)))
    (Audio|Components|Audio|Play _skeletalmesh false)))