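; Interactable cage holding a weasel creature that gets released through an airlock when activated.
; A player-tagged actor entering the box trigger sets the Enter flag on the creature's AB_Weasle anim instance.
; Activate runs the parent logic, then OpenAirlock plays the airlock after a delay.
; After a further delay, the creature switches to physics simulation and receives a small backward impulse.
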(event OnComponentBeginOverlap(Box)
  (params (OverlappedComponent :type Primitive%20Component%20Object%20Reference) (OtherActor :type Actor%20Object%20Reference) (OtherComp :type Primitive%20Component%20Object%20Reference) (OtherBodyIndex :type Integer) (bFromSweep :type Boolean) (SweepResult :type Hit%20Result%20Structure%20%28by%20ref%29))
  (if (Actor|ActorHasTag OtherActor "player")
    (bind _asab_weasle (Utilities|Casting|CastToAB_Weasle (Components|SkeletalMesh|GetAnimInstance (Variables|Default|GetCreature))))
    (Variables|/Game/Meshes/Animations/Pet/AB_Weasle.AB_Weasle_C|Setenter _asab_weasle true)))

(event Custom|Open%20Airlock
  (bind _creature (Variables|Default|GetCreature))
  (Utilities|FlowControl|Delay 2.0)
  (Audio|Components|Audio|Play (Variables|Default|GetAirlock) false)
  (Utilities|FlowControl|Delay 1.2)
  (Collision|SetCollisionEnabled _creature "PhysicsOnly")
  (Physics|SetSimulatePhysics _creature true)
  (Physics|AddImpulse _creature (* (* (Math|Vector|GetForwardVector (Variables|Default|GetCreature)) -1.0) 1.0) "None" false))

(event EventTick
  (params (DeltaSeconds :type Float%20%28single-precision%29))
  (|CallParentFunction DeltaSeconds) ; This node is disabled and will not be called.\nDrag off pins to build functionality.
)

(fn ConstructionScript
  (|CallParentFunction))

(fn Activate
  (|CallParentFunction)
  (CallFunction|OpenAirlock))