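; Interactable that triggers a self-destruct sequence ending the game when activated.
; Activate calls the parent, then raises a warning-light parameter in a material parameter collection and plays the self-destruct sound.
; After a timed delay it activates the explosion particle system and sound, then quits the game shortly after.
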(event Custom|Initiate%20Self%20Destruction
  (bind _audio (Variables|Default|GetAudio))
  (bind _audio_2 (Variables|Default|GetAudio))
  (Rendering|Material|SetScalarParameterValue "/Game/MPC_WarningLight.MPC_WarningLight" "R5_warningLight" 1.0 :!class /Script/Engine.KismetMaterialLibrary)
  (Audio|Components|Audio|SetSound _audio_2 "/Game/Audio/SelfDestruct_Cue.SelfDestruct_Cue")
  (Audio|Components|Audio|Play _audio_2 0.0)
  (Utilities|FlowControl|Delay 11.3)
  (Components|Activation|Activate (Variables|Default|GetParticleSystem) true)
  (Audio|Components|Audio|SetSound _audio "/Game/StarterContent/Audio/Explosion_Cue.Explosion_Cue")
  (Audio|Components|Audio|Play _audio 0.0)
  (Utilities|FlowControl|Delay 0.5)
  (Game|QuitGame 0 "Quit" false))

(fn ConstructionScript
  (|CallParentFunction))

(fn Activate
  (|CallParentFunction)
  (CallFunction|InitiateSelfDestruction))