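; BP_Seed is a seed actor that the player picks up and carries in first-person view when activated.
; Its Activate override calls the parent, then proceeds only if the player character's PickedSeed slot is empty, storing itself there.
; It snaps to the SeedHolder's transform, attaches to the first-person camera keeping that world transform, and disables collision and shadow casting on its root.
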(event EventBeginPlay
  (|CallParentFunction) ; This node is disabled and will not be called.\nDrag off pins to build functionality.
)

(event Collision|EventActorBeginOverlap
  (params (OtherActor :type Actor%20Object%20Reference))
  (|CallParentFunction OtherActor) ; This node is disabled and will not be called.\nDrag off pins to build functionality.
)

(event EventTick
  (params (DeltaSeconds :type Float%20%28single-precision%29))
  (|CallParentFunction DeltaSeconds) ; This node is disabled and will not be called.\nDrag off pins to build functionality.
)

(fn ConstructionScript
  (|CallParentFunction))

(fn Activate
  (bind _root (Variables|Default|GetRoot))
  (|CallParentFunction)
  (bind _asfirst_person_character (Utilities|Casting|CastToFirstPersonCharacter (Game|GetPlayerCharacter 0)))
  (if (== (Variables|/Game/FirstPersonBP/Blueprints/FirstPersonCharacter.FirstPersonCharacter_C|GetpickedSeed _asfirst_person_character) 0)
    (Variables|/Game/FirstPersonBP/Blueprints/FirstPersonCharacter.FirstPersonCharacter_C|SetpickedSeed _asfirst_person_character self)
    (Transformation|SetActorLocation (Transformation|GetWorldLocation (Variables|/Game/FirstPersonBP/Blueprints/FirstPersonCharacter.FirstPersonCharacter_C|GetSeedHolder _asfirst_person_character)) false false)
    (Transformation|SetActorRotation (Transformation|GetWorldRotation (Variables|/Game/FirstPersonBP/Blueprints/FirstPersonCharacter.FirstPersonCharacter_C|GetSeedHolder _asfirst_person_character)))
    (Transformation|SetActorScale3D (Transformation|GetWorldScale (Variables|/Game/FirstPersonBP/Blueprints/FirstPersonCharacter.FirstPersonCharacter_C|GetSeedHolder _asfirst_person_character)))
    (Transformation|AttachComponentToComponent (Variables|/Game/FirstPersonBP/Blueprints/FirstPersonCharacter.FirstPersonCharacter_C|GetFirstPersonCamera _asfirst_person_character) "None" "KeepWorld" "KeepWorld" "KeepWorld" true)
    (Collision|SetCollisionEnabled _root "NoCollision")
    (Rendering|SetCastShadow _root false)))